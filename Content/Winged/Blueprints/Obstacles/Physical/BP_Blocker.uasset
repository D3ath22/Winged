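; BP_Blocker is a physical obstacle that stuns Kora or Kayn on impact and then destroys itself.
; The Blocker component's hit event identifies the character by cast and does nothing if that character's shield is valid.
; Each stun also appends time, player location, current respawn location and blocker name to the singleplayer interaction events in the save game object, reached through the game instance cached on BeginPlay.
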(event `self.ReceiveBeginPlay`
  (bind _aswinged_game_instance (cast `/Game/Winged/Blueprints/WingedGameInstance` (`GameplayStatics.GetGameInstance`)))
  (set `self.GameInstance` _aswinged_game_instance))

(event `self.Blocker.OnComponentHit`
  (params (HitComponent :type "PrimitiveComponent Object Reference") (OtherActor :type "Actor Object Reference") (OtherComp :type "PrimitiveComponent Object Reference") (NormalImpulse :type "Vector Structure") (Hit :type "HitResult Structure (by ref)"))
  (bind _askora (cast `/Game/Winged/Blueprints/Kora` OtherActor)
    (:`then`
      (if (not (`KismetSystemLibrary.IsValid` (`/Game/Winged/Blueprints/Kora.KoraShield` _askora)))
        (`/Game/Winged/Blueprints/Kora.Stun` _askora)
        (`self.K2_DestroyActor`)
        (`KismetArrayLibrary.Array_Add` (`/Game/Winged/Blueprints/WingedSaveGame.Events_SingleplayerInteraction` (`/Game/Winged/Blueprints/WingedGameInstance.SaveGame` (`self.GameInstance`))) (make `/Game/Winged/Blueprints/Structure_Event` (`KismetSystemLibrary.GetGameTimeInSeconds`) (`self.K2_GetActorLocation` _askora) (`/Game/Winged/Blueprints/Kora.CurrentRespawnLocation` _askora) (`KismetSystemLibrary.GetDisplayName` self)))))
    (:`CastFailed`
      (bind _askayn (cast `/Game/Winged/Blueprints/Kayn` OtherActor))
      (if (not (`KismetSystemLibrary.IsValid` (`/Game/Winged/Blueprints/Kayn.KaynShield` _askayn)))
        (`/Game/Winged/Blueprints/Kayn.Stun` _askayn)
        (`self.K2_DestroyActor`)
        (`KismetArrayLibrary.Array_Add` (`/Game/Winged/Blueprints/WingedSaveGame.Events_SingleplayerInteraction` (`/Game/Winged/Blueprints/WingedGameInstance.SaveGame` (`self.GameInstance`))) (make `/Game/Winged/Blueprints/Structure_Event` (`KismetSystemLibrary.GetGameTimeInSeconds`) (`self.K2_GetActorLocation` _askayn) (`/Game/Winged/Blueprints/Kayn.CurrentRespawnLocation` _askayn) (`KismetSystemLibrary.GetDisplayName` self)))))))

(fn `UserConstructionScript`)