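; Griffon-animated spirit obstacle that Kora or Kayn can convert for a spirit count and a temporary speed boost.
; It wanders via AIMoveTo between random TargetPoints tagged with its display name until converted.
; The players' convert dispatchers trigger Purify or Radicalize, which match the overlapped name, log the conversion to the save game, or stun a rival converting an owned spirit.
; Once converted, it casts its side's spell once in multiplayer; its overlap logic is disconnected.
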(event `self.ReceiveBeginPlay`
  (bind _returnvalue (`GameplayStatics.GetPlayerPawn` 1))
  (bind _returnvalue_2 (`GameplayStatics.GetPlayerPawn` 0))
  (bind _targets (`self.Targets`))
  (set `CharacterMovementComponent.bOrientRotationToMovement` true (`self.CharacterMovement`))
  (`CharacterMovementComponent.SetMovementMode` (`self.CharacterMovement`) "MOVE_NavWalking" 0)
  (bind _outactors (`GameplayStatics.GetAllActorsWithTag` (`KismetStringLibrary.Conv_StringToName` (`KismetSystemLibrary.GetDisplayName` self))))
  (for _array_element _outactors
    (bind _astarget_point (cast `TargetPoint` _array_element))
    (`KismetArrayLibrary.Array_Add` (`self.Targets`) _astarget_point))
  (set `self.CurrentTarget` (`|GetArrayItem` _targets (`KismetMathLibrary.RandomIntegerInRange` 0 (`KismetArrayLibrary.Array_LastIndex` _targets))))
  (bind _askora (cast `/Game/Winged/Blueprints/Kora` _returnvalue_2)
    (:`then`
      (bind _output_get (set `self.PawnKora` _askora))
      (add `/Game/Winged/Blueprints/Kora.Dispatcher_KoraConvert` _output_get (delegate `Purify`)))
    (:`CastFailed`
      (bind _askayn (cast `/Game/Winged/Blueprints/Kayn` _returnvalue_2))
      (bind _output_get_2 (set `self.PawnKayn` _askayn))
      (add `/Game/Winged/Blueprints/Kayn.Dispatcher_KaynConvert` _output_get_2 (delegate `Radicalize`))))
  (bind _aswinged_game_instance (cast `/Game/Winged/Blueprints/WingedGameInstance` (`GameplayStatics.GetGameInstance`)))
  (set `self.GameInstance` _aswinged_game_instance)
  (if (not (`/Game/Winged/Blueprints/WingedGameInstance.SinglePlayer` _aswinged_game_instance))
    (bind _askora_2 (cast `/Game/Winged/Blueprints/Kora` _returnvalue)
      (:`then`
        (bind _output_get_3 (set `self.PawnKora` _askora_2))
        (add `/Game/Winged/Blueprints/Kora.Dispatcher_KoraConvert` _output_get_3 (delegate `Purify`)))
      (:`CastFailed`
        (bind _askayn_2 (cast `/Game/Winged/Blueprints/Kayn` _returnvalue))
        (bind _output_get_4 (set `self.PawnKayn` _askayn_2))
        (add `/Game/Winged/Blueprints/Kayn.Dispatcher_KaynConvert` _output_get_4 (delegate `Radicalize`))))))

(event `Purify`
  (bind _pawnkora (`self.PawnKora`))
  (bind _pawnkora_2 (`self.PawnKora`))
  (bind (_returnvalue_x _returnvalue_y _returnvalue_z) (`KismetMathLibrary.BreakVector` (`SceneComponent.K2_GetComponentLocation` (`self.Capsule`))))
  (if (`KismetStringLibrary.EqualEqual_StrStr` (`/Game/Winged/Blueprints/Kora.OverlappingName` _pawnkora_2) (`KismetSystemLibrary.GetObjectName` self))
    (if (`self.Converted`)
      (if (not (`self.KoraConverted`))
        (`/Game/Winged/Blueprints/Kora.Stun` (`self.PawnKora`))
        (`SkeletalMeshComponent.PlayAnimation` (`self.Mesh`) "/Game/UsedAssets/QuadrapedCreatures/Griffon/Animations/ANIM_Griffon_BiteAttack.ANIM_Griffon_BiteAttack" false))
      (else
        (`KismetArrayLibrary.Array_Add` (`/Game/Winged/Blueprints/WingedSaveGame.Events_SingleplayerInteraction` (`/Game/Winged/Blueprints/WingedGameInstance.SaveGame` (`self.GameInstance`))) (make `/Game/Winged/Blueprints/Structure_Event` (`KismetSystemLibrary.GetGameTimeInSeconds`) (`self.K2_GetActorLocation`) (`/Game/Winged/Blueprints/Kora.CurrentRespawnLocation` _pawnkora_2) (`KismetSystemLibrary.GetDisplayName` self)))
        (`SkeletalMeshComponent.PlayAnimation` (`self.Mesh`) "/Game/UsedAssets/QuadrapedCreatures/Griffon/Animations/ANIM_Griffon_Landing.ANIM_Griffon_Landing" false)
        (`GameplayStatics.PlaySoundAtLocation` "/Game/Winged/Assets/HighFiveEffect/Sound_HighFive_Cue.Sound_HighFive_Cue" (`self.K2_GetActorLocation` (`self.PawnKora`)) (struct) 1.0 1.0 0.0 null null null)
        (`|SpawnActorFromClass` "/Game/Winged/Blueprints/Effects/BP_AuraEffect_Kora.BP_AuraEffect_Kora_C" (`KismetMathLibrary.MakeTransform` (`KismetMathLibrary.MakeVector` _returnvalue_x _returnvalue_y _returnvalue_z)) "Undefined" "OverrideRootScale" self null)
        (`/Game/Winged/Blueprints/Kora.AddSpirit` _pawnkora)
        (set `self.Converted` true)
        (set `self.KoraConverted` true)
        (bind _msbuff (`/Game/Winged/Blueprints/Kora.AddMovementSpeedBoost` _pawnkora))
        (bind _aswinged_game_instance (cast `/Game/Winged/Blueprints/WingedGameInstance` (`GameplayStatics.GetGameInstance`)))
        (`KismetSystemLibrary.Delay` (`/Game/Winged/Blueprints/WingedGameInstance.MovementSpeedBoostDuration` _aswinged_game_instance))
        (`/Game/Winged/Blueprints/Kora.RemoveMovementSpeedBoost` _pawnkora _msbuff)))))

(event `Radicalize`
  (bind _pawnkayn (`self.PawnKayn`))
  (bind _pawnkayn_2 (`self.PawnKayn`))
  (bind (_returnvalue_x _returnvalue_y _returnvalue_z) (`KismetMathLibrary.BreakVector` (`SceneComponent.K2_GetComponentLocation` (`self.Capsule`))))
  (if (`KismetStringLibrary.EqualEqual_StrStr` (`/Game/Winged/Blueprints/Kayn.OverlappingName` _pawnkayn) (`KismetSystemLibrary.GetObjectName` self))
    (if (`self.Converted`)
      (if (`self.KoraConverted`)
        (`/Game/Winged/Blueprints/Kayn.Stun` (`self.PawnKayn`))
        (`SkeletalMeshComponent.PlayAnimation` (`self.Mesh`) "/Game/UsedAssets/QuadrapedCreatures/Griffon/Animations/ANIM_Griffon_BiteAttack.ANIM_Griffon_BiteAttack" false))
      (else
        (`KismetArrayLibrary.Array_Add` (`/Game/Winged/Blueprints/WingedSaveGame.Events_SingleplayerInteraction` (`/Game/Winged/Blueprints/WingedGameInstance.SaveGame` (`self.GameInstance`))) (make `/Game/Winged/Blueprints/Structure_Event` (`KismetSystemLibrary.GetGameTimeInSeconds`) (`self.K2_GetActorLocation`) (`/Game/Winged/Blueprints/Kayn.CurrentRespawnLocation` _pawnkayn) (`KismetSystemLibrary.GetDisplayName` self)))
        (`SkeletalMeshComponent.PlayAnimation` (`self.Mesh`) "/Game/UsedAssets/QuadrapedCreatures/Griffon/Animations/ANIM_Griffon_Landing.ANIM_Griffon_Landing" false)
        (`GameplayStatics.PlaySoundAtLocation` "/Game/Winged/Assets/HighFiveEffect/Sound_HighFive_Cue.Sound_HighFive_Cue" (`self.K2_GetActorLocation` (`self.PawnKayn`)) (struct) 1.0 1.0 0.0 null null null)
        (`|SpawnActorFromClass` "/Game/Winged/Blueprints/Effects/BP_AuraEffect_Kayn.BP_AuraEffect_Kayn_C" (`KismetMathLibrary.MakeTransform` (`KismetMathLibrary.MakeVector` _returnvalue_x _returnvalue_y _returnvalue_z)) "Undefined" "OverrideRootScale" self null)
        (`/Game/Winged/Blueprints/Kayn.AddSpirit` _pawnkayn_2)
        (set `self.Converted` true)
        (set `self.KoraConverted` false)
        (bind _msbuff (`/Game/Winged/Blueprints/Kayn.AddMovementSpeedBoost` _pawnkayn_2))
        (bind _aswinged_game_instance (cast `/Game/Winged/Blueprints/WingedGameInstance` (`GameplayStatics.GetGameInstance`)))
        (`KismetSystemLibrary.Delay` (`/Game/Winged/Blueprints/WingedGameInstance.MovementSpeedBoostDuration` _aswinged_game_instance))
        (`/Game/Winged/Blueprints/Kayn.RemoveMovementSpeedBoost` _pawnkayn_2 _msbuff)))))

(event `self.Capsule.OnComponentBeginOverlap`
  (params (OverlappedComponent :type "PrimitiveComponent Object Reference") (OtherActor :type "Actor Object Reference") (OtherComp :type "PrimitiveComponent Object Reference") (OtherBodyIndex :type Integer) (bFromSweep :type Boolean) (SweepResult :type "HitResult Structure (by ref)")))

(event `self.Capsule.OnComponentEndOverlap`
  (params (OverlappedComponent :type "PrimitiveComponent Object Reference") (OtherActor :type "Actor Object Reference") (OtherComp :type "PrimitiveComponent Object Reference") (OtherBodyIndex :type Integer)))

(event `self.ReceiveTick`
  (params (DeltaSeconds :type "Float (single-precision)"))
  (bind _targets (`self.Targets`))
  (bind (_returnvalue_x _returnvalue_y _returnvalue_z) (`KismetMathLibrary.BreakVector` (`SceneComponent.K2_GetComponentLocation` (`self.CapsuleComponent`))))
  (bind (_returnvalue_x_2 _returnvalue_y_2 _returnvalue_z_2) (`KismetMathLibrary.BreakVector` (`SceneComponent.K2_GetComponentLocation` (`self.CapsuleComponent`))))
  (bind _aswinged_game_instance (cast `/Game/Winged/Blueprints/WingedGameInstance` (`GameplayStatics.GetGameInstance`) :!pure true))
  (if (not (`self.Overlapping`))
    (`KismetSystemLibrary.Delay` 2.0)
    (`SkeletalMeshComponent.PlayAnimation` (`self.Mesh`) "/Game/UsedAssets/QuadrapedCreatures/Griffon/Animations/ANIM_Griffon_FlyNormal.ANIM_Griffon_FlyNormal" true)
    (if (`self.Converted`)
      (`/Engine/EditorBlueprintResources/StandardMacros.DoOnce` false
        (:`Completed`
          (if (and (`self.KoraConverted`) (== (`/Game/Winged/Blueprints/WingedGameInstance.SinglePlayer` _aswinged_game_instance) false))
            (`GameplayStatics.PlaySoundAtLocation` "/Game/Winged/Assets/AuraEffect/Sound_Spell_Cue.Sound_Spell_Cue" (`self.K2_GetActorLocation`) (struct) 1.0 1.0 0.0 null null null)
            (`|SpawnActorFromClass` "/Game/Winged/Blueprints/Effects/BP_Spell_KoraSpirit.BP_Spell_KoraSpirit_C" (`KismetMathLibrary.MakeTransform` (`KismetMathLibrary.MakeVector` (+ _returnvalue_x_2 20.0) _returnvalue_y_2 _returnvalue_z_2) (`self.GetControlRotation` self)) "Undefined" "OverrideRootScale" self null)
            (elif (and (== (`self.KoraConverted`) false) (== (`/Game/Winged/Blueprints/WingedGameInstance.SinglePlayer` _aswinged_game_instance) false))
              (`GameplayStatics.PlaySoundAtLocation` "/Game/Winged/Assets/AuraEffect/Sound_Spell_Cue.Sound_Spell_Cue" (`self.K2_GetActorLocation`) (struct) 1.0 1.0 0.0 null null null)
              (`|SpawnActorFromClass` "/Game/Winged/Blueprints/Effects/BP_Spell_KaynSpirit.BP_Spell_KaynSpirit_C" (`KismetMathLibrary.MakeTransform` (`KismetMathLibrary.MakeVector` (+ _returnvalue_x 20.0) _returnvalue_y _returnvalue_z) (`self.GetControlRotation` self)) "Undefined" "OverrideRootScale" self null)))))
      (else
        (`|AIMoveTo` self (`self.K2_GetActorLocation` (`self.CurrentTarget`)) null
          (:`then`
            (`KismetSystemLibrary.Delay` 1.0)
            (set `self.CurrentTarget` (`|GetArrayItem` _targets (`KismetMathLibrary.RandomIntegerInRange` 0 (`KismetArrayLibrary.Array_LastIndex` _targets))))))))))

(fn `UserConstructionScript`)