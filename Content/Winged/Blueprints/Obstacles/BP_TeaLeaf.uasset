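; BP_TeaLeaf is a one-shot pickup that rewards Kora with energy and a timed speed boost, or lets Kayn deny it.
; Capsule overlap plays a sound, hides the leaf and disables collision for either character.
; For Kora it also logs the interaction to the SaveGame, then stays alive through the GameInstance-defined boost duration to remove the boost before destroying itself.
; For Kayn it calls AddKoraEnergyDenied and destroys itself immediately.
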(event `self.ReceiveBeginPlay`
  (bind _aswinged_game_instance (cast `/Game/Winged/Blueprints/WingedGameInstance` (`GameplayStatics.GetGameInstance`)))
  (set `self.GameInstance` _aswinged_game_instance))

(event `self.Capsule.OnComponentBeginOverlap`
  (params (OverlappedComponent :type "PrimitiveComponent Object Reference") (OtherActor :type "Actor Object Reference") (OtherComp :type "PrimitiveComponent Object Reference") (OtherBodyIndex :type Integer) (bFromSweep :type Boolean) (SweepResult :type "HitResult Structure (by ref)"))
  (bind _askora (cast `/Game/Winged/Blueprints/Kora` OtherActor)
    (:`then`
      (`KismetArrayLibrary.Array_Add` (`/Game/Winged/Blueprints/WingedSaveGame.Events_SingleplayerInteraction` (`/Game/Winged/Blueprints/WingedGameInstance.SaveGame` (`self.GameInstance`))) (make `/Game/Winged/Blueprints/Structure_Event` (`KismetSystemLibrary.GetGameTimeInSeconds`) (`self.K2_GetActorLocation`) (`/Game/Winged/Blueprints/Kora.CurrentRespawnLocation` _askora) (`KismetSystemLibrary.GetDisplayName` self)))
      (`GameplayStatics.PlaySoundAtLocation` "/Game/Winged/Assets/KaynEnergySound/Sound_KaynEnergy_Pickup_Cue.Sound_KaynEnergy_Pickup_Cue" (`self.K2_GetActorLocation`) (struct) 1.0 1.0 0.0 null null null)
      (`SceneComponent.SetVisibility` (`self.DefaultSceneRoot`) false true)
      (`self.SetActorEnableCollision` false)
      (`/Game/Winged/Blueprints/Kora.AddKoraEnergy` _askora)
      (bind _msbuff (`/Game/Winged/Blueprints/Kora.AddMovementSpeedBoost` _askora))
      (bind _aswinged_game_instance (cast `/Game/Winged/Blueprints/WingedGameInstance` (`GameplayStatics.GetGameInstance`)))
      (`KismetSystemLibrary.Delay` (`/Game/Winged/Blueprints/WingedGameInstance.MovementSpeedBoostDuration` _aswinged_game_instance))
      (`/Game/Winged/Blueprints/Kora.RemoveMovementSpeedBoost` _askora _msbuff)
      (`self.K2_DestroyActor`))
    (:`CastFailed`
      (bind _askayn (cast `/Game/Winged/Blueprints/Kayn` OtherActor))
      (`GameplayStatics.PlaySoundAtLocation` "/Game/Winged/Assets/KaynEnergySound/Sound_KaynEnergy_Pickup_Cue.Sound_KaynEnergy_Pickup_Cue" (`self.K2_GetActorLocation`) (struct) 1.0 1.0 0.0 null null null)
      (`SceneComponent.SetVisibility` (`self.DefaultSceneRoot`) false true)
      (`self.SetActorEnableCollision` false)
      (`/Game/Winged/Blueprints/Kayn.AddKoraEnergyDenied` _askayn)
      (`self.K2_DestroyActor`))))

(fn `UserConstructionScript`)