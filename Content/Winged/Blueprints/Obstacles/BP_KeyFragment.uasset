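; Key fragment that acts as the level goal for the two characters, Kora and Kayn.
; On overlap it records the character's finish time and adds an interaction event to the save game object.
; The first arrival sets the winner in WingedGameInstance, winning if within the level one time limit or untimed, otherwise losing to the other.
; Each overlapping character gets its own transition menu, and player 0's mouse cursor is shown.
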(event `self.ReceiveBeginPlay`
  (bind _aswinged_game_instance (cast `/Game/Winged/Blueprints/WingedGameInstance` (`GameplayStatics.GetGameInstance`)))
  (set `self.GameInstance` _aswinged_game_instance))

(event `self.KeyFragment.OnComponentBeginOverlap`
  (params (OverlappedComponent :type "PrimitiveComponent Object Reference") (OtherActor :type "Actor Object Reference") (OtherComp :type "PrimitiveComponent Object Reference") (OtherBodyIndex :type Integer) (bFromSweep :type Boolean) (SweepResult :type "HitResult Structure (by ref)"))
  (bind _returnvalue (`KismetSystemLibrary.GetGameTimeInSeconds`))
  (bind _gameinstance (`self.GameInstance`))
  (bind _gameinstance_2 (`self.GameInstance`))
  (bind _askora (cast `/Game/Winged/Blueprints/Kora` OtherActor)
    (:`then`
      (bind _output_get (set `/Game/Winged/Blueprints/Kora.FinishTIme` _returnvalue _askora))
      (`KismetArrayLibrary.Array_Add` (`/Game/Winged/Blueprints/WingedSaveGame.Events_SingleplayerInteraction` (`/Game/Winged/Blueprints/WingedGameInstance.SaveGame` (`self.GameInstance`))) (make `/Game/Winged/Blueprints/Structure_Event` _output_get (`self.K2_GetActorLocation`) 0 (`KismetSystemLibrary.GetDisplayName` self)))
      (if (not (`/Game/Winged/Blueprints/WingedGameInstance.EndReached` _gameinstance_2))
        (if (or (<= (`/Game/Winged/Blueprints/Kora.FinishTIme` _askora) (`KismetMathLibrary.Conv_IntToDouble` (`/Game/Winged/Blueprints/WingedGameInstance.LevelOne_TimeMax` _gameinstance_2))) (`/Game/Winged/Blueprints/WingedGameInstance.NoTimeLimit` _gameinstance_2))
          (set `/Game/Winged/Blueprints/WingedGameInstance.KoraWin` true _gameinstance_2)
          (else
            (set `/Game/Winged/Blueprints/WingedGameInstance.KoraWin` false _gameinstance_2)))
        (set `/Game/Winged/Blueprints/WingedGameInstance.EndReached` true _gameinstance_2))
      (bind _asplayer_controller (cast `PlayerController` (`Pawn.GetController` _askora)))
      (bind _returnvalue_2 (`|CreateWidget` "/Game/Winged/Blueprints/TransitionMenu/KoraTransitionMenuWidget.KoraTransitionMenuWidget_C" _asplayer_controller))
      (`UserWidget.AddToPlayerScreen` _returnvalue_2 0)
      (set `PlayerController.bShowMouseCursor` true (`GameplayStatics.GetPlayerController` 0)))
    (:`CastFailed`
      (bind _askayn (cast `/Game/Winged/Blueprints/Kayn` OtherActor))
      (bind _output_get_2 (set `/Game/Winged/Blueprints/Kayn.FinishTime` _returnvalue _askayn))
      (`KismetArrayLibrary.Array_Add` (`/Game/Winged/Blueprints/WingedSaveGame.Events_SingleplayerInteraction` (`/Game/Winged/Blueprints/WingedGameInstance.SaveGame` (`self.GameInstance`))) (make `/Game/Winged/Blueprints/Structure_Event` _output_get_2 (`self.K2_GetActorLocation`) (`/Game/Winged/Blueprints/Kayn.CurrentRespawnLocation` _askayn) (`KismetSystemLibrary.GetDisplayName` self)))
      (if (not (`/Game/Winged/Blueprints/WingedGameInstance.EndReached` _gameinstance))
        (if (or (<= (`/Game/Winged/Blueprints/Kayn.FinishTime` _askayn) (`KismetMathLibrary.Conv_IntToDouble` (`/Game/Winged/Blueprints/WingedGameInstance.LevelOne_TimeMax` _gameinstance))) (`/Game/Winged/Blueprints/WingedGameInstance.NoTimeLimit` _gameinstance))
          (set `/Game/Winged/Blueprints/WingedGameInstance.KoraWin` false _gameinstance)
          (else
            (set `/Game/Winged/Blueprints/WingedGameInstance.KoraWin` true _gameinstance)))
        (set `/Game/Winged/Blueprints/WingedGameInstance.EndReached` true _gameinstance))
      (bind _asplayer_controller_2 (cast `PlayerController` (`Pawn.GetController` _askayn)))
      (bind _returnvalue_3 (`|CreateWidget` "/Game/Winged/Blueprints/TransitionMenu/KaynTransitionMenuWidget.KaynTransitionMenuWidget_C" _asplayer_controller_2))
      (`UserWidget.AddToPlayerScreen` _returnvalue_3 0)
      (set `PlayerController.bShowMouseCursor` true (`GameplayStatics.GetPlayerController` 0)))))

(fn `UserConstructionScript`)