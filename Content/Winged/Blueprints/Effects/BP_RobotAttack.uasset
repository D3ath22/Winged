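; BP_RobotAttack is an attack effect actor that plays the robot attack sound on spawn and stuns the player characters Kora or Kayn on contact.
; The Attack component's overlap logs time, location, respawn point and actor name to the SaveGame's singleplayer interaction events, even for shielded players.
; Without a valid shield, the character is stunned and the actor destroys itself after a short delay.
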(event `self.ReceiveBeginPlay`
  (`GameplayStatics.PlaySoundAtLocation` "/Game/Winged/Assets/RobotEffect_Attack/Sound_RobotAttack_Cue.Sound_RobotAttack_Cue" (`self.K2_GetActorLocation`) (struct) 1.0 1.0 0.0 null null null))

(event `self.Attack.OnComponentBeginOverlap`
  (params (OverlappedComponent :type "PrimitiveComponent Object Reference") (OtherActor :type "Actor Object Reference") (OtherComp :type "PrimitiveComponent Object Reference") (OtherBodyIndex :type Integer) (bFromSweep :type Boolean) (SweepResult :type "HitResult Structure (by ref)"))
  (bind _aswinged_game_instance (cast `/Game/Winged/Blueprints/WingedGameInstance` (`GameplayStatics.GetGameInstance`) :!pure true))
  (bind _askora (cast `/Game/Winged/Blueprints/Kora` OtherActor)
    (:`then`
      (`KismetArrayLibrary.Array_Add` (`/Game/Winged/Blueprints/WingedSaveGame.Events_SingleplayerInteraction` (`/Game/Winged/Blueprints/WingedGameInstance.SaveGame` _aswinged_game_instance)) (make `/Game/Winged/Blueprints/Structure_Event` (`KismetSystemLibrary.GetGameTimeInSeconds`) (`self.K2_GetActorLocation`) (`/Game/Winged/Blueprints/Kora.CurrentRespawnLocation` _askora) (`KismetSystemLibrary.GetDisplayName` self)))
      (if (not (`KismetSystemLibrary.IsValid` (`/Game/Winged/Blueprints/Kora.KoraShield` _askora)))
        (`/Game/Winged/Blueprints/Kora.Stun` _askora)
        (`KismetSystemLibrary.Delay` 2.0)
        (`self.K2_DestroyActor`)))
    (:`CastFailed`
      (bind _askayn (cast `/Game/Winged/Blueprints/Kayn` OtherActor))
      (`KismetArrayLibrary.Array_Add` (`/Game/Winged/Blueprints/WingedSaveGame.Events_SingleplayerInteraction` (`/Game/Winged/Blueprints/WingedGameInstance.SaveGame` _aswinged_game_instance)) (make `/Game/Winged/Blueprints/Structure_Event` (`KismetSystemLibrary.GetGameTimeInSeconds`) (`self.K2_GetActorLocation`) (`/Game/Winged/Blueprints/Kayn.CurrentRespawnLocation` _askayn) (`KismetSystemLibrary.GetDisplayName` self)))
      (if (not (`KismetSystemLibrary.IsValid` (`/Game/Winged/Blueprints/Kayn.KaynShield` _askayn)))
        (`/Game/Winged/Blueprints/Kayn.Stun` _askayn)
        (`KismetSystemLibrary.Delay` 2.0)
        (`self.K2_DestroyActor`)))))

(fn `UserConstructionScript`)