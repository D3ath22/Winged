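; BP_Spell_KaynSpirit is a homing spell projectile owned by BP_Spirit that stuns Kora on contact.
; On BeginPlay it homes on the capsule of the spirit's PawnKora with high acceleration, then destroys itself after a fixed delay.
; An Aura overlap with Kora stuns her, logs time, location, respawn point and spell name to the save game's multiplayer interaction events, then destroys the spell.
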(event `self.ReceiveBeginPlay`
  (bind _projectilemovement (`self.ProjectileMovement`))
  (bind _asbp_spirit (cast `/Game/Winged/Blueprints/Obstacles/BP_Spirit` (`self.GetOwner`)))
  (set `ProjectileMovementComponent.HomingTargetComponent` (`Character.CapsuleComponent` (`/Game/Winged/Blueprints/Obstacles/BP_Spirit.PawnKora` _asbp_spirit)) _projectilemovement)
  (set `ProjectileMovementComponent.bIsHomingProjectile` true _projectilemovement)
  (set `ProjectileMovementComponent.HomingAccelerationMagnitude` 10000.0 _projectilemovement)
  (`KismetSystemLibrary.Delay` 5.0)
  (`self.K2_DestroyActor`))

(event `self.Aura.OnComponentBeginOverlap`
  (params (OverlappedComponent :type "PrimitiveComponent Object Reference") (OtherActor :type "Actor Object Reference") (OtherComp :type "PrimitiveComponent Object Reference") (OtherBodyIndex :type Integer) (bFromSweep :type Boolean) (SweepResult :type "HitResult Structure (by ref)"))
  (bind _askora (cast `/Game/Winged/Blueprints/Kora` OtherActor))
  (`/Game/Winged/Blueprints/Kora.Stun` _askora)
  (`KismetArrayLibrary.Array_Add` (`/Game/Winged/Blueprints/WingedSaveGame.Events_MultiplayerInteraction` (`/Game/Winged/Blueprints/WingedGameInstance.SaveGame` (cast `/Game/Winged/Blueprints/WingedGameInstance` (`GameplayStatics.GetGameInstance`) :!pure true))) (make `/Game/Winged/Blueprints/Structure_Event` (`KismetSystemLibrary.GetGameTimeInSeconds`) (`self.K2_GetActorLocation`) (`/Game/Winged/Blueprints/Kora.CurrentRespawnLocation` _askora) (`KismetSystemLibrary.GetDisplayName` self)))
  (`self.K2_DestroyActor`))

(fn `UserConstructionScript`)