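; Kora's spell actor, a short-lived aura that counters Kayn and his spells and destroys itself three seconds after spawning.
; On Aura overlap, a cast chain stuns Kayn or destroys a BP_Spell_Kayn or BP_Spell_KaynSpirit.
; Each hit appends time, spell location, owner Kora's respawn location and both display names to the save game's multiplayer interaction events.
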(event `self.ReceiveBeginPlay`
  (`KismetSystemLibrary.Delay` 3.0)
  (`self.K2_DestroyActor`))

(event `self.Aura.OnComponentBeginOverlap`
  (params (OverlappedComponent :type "PrimitiveComponent Object Reference") (OtherActor :type "Actor Object Reference") (OtherComp :type "PrimitiveComponent Object Reference") (OtherBodyIndex :type Integer) (bFromSweep :type Boolean) (SweepResult :type "HitResult Structure (by ref)"))
  (bind _askayn (cast `/Game/Winged/Blueprints/Kayn` OtherActor)
    (:`then`
      (`/Game/Winged/Blueprints/Kayn.Stun` _askayn)
      (`KismetArrayLibrary.Array_Add` (`/Game/Winged/Blueprints/WingedSaveGame.Events_MultiplayerInteraction` (`/Game/Winged/Blueprints/WingedGameInstance.SaveGame` (cast `/Game/Winged/Blueprints/WingedGameInstance` (`GameplayStatics.GetGameInstance`) :!pure true))) (make `/Game/Winged/Blueprints/Structure_Event` (`KismetSystemLibrary.GetGameTimeInSeconds`) (`self.K2_GetActorLocation`) (`/Game/Winged/Blueprints/Kora.CurrentRespawnLocation` (cast `/Game/Winged/Blueprints/Kora` (`self.GetOwner`) :!pure true)) (`KismetStringLibrary.Concat_StrStr` (`KismetSystemLibrary.GetDisplayName` self) (`KismetSystemLibrary.GetDisplayName` _askayn)))))
    (:`CastFailed`
      (bind _asbp_spell_kayn (cast `/Game/Winged/Blueprints/Effects/BP_Spell_Kayn` OtherActor)
        (:`then`
          (`self.K2_DestroyActor` _asbp_spell_kayn)
          (`KismetArrayLibrary.Array_Add` (`/Game/Winged/Blueprints/WingedSaveGame.Events_MultiplayerInteraction` (`/Game/Winged/Blueprints/WingedGameInstance.SaveGame` (cast `/Game/Winged/Blueprints/WingedGameInstance` (`GameplayStatics.GetGameInstance`) :!pure true))) (make `/Game/Winged/Blueprints/Structure_Event` (`KismetSystemLibrary.GetGameTimeInSeconds`) (`self.K2_GetActorLocation`) (`/Game/Winged/Blueprints/Kora.CurrentRespawnLocation` (cast `/Game/Winged/Blueprints/Kora` (`self.GetOwner`) :!pure true)) (`KismetStringLibrary.Concat_StrStr` (`KismetSystemLibrary.GetDisplayName` self) (`KismetSystemLibrary.GetDisplayName` _asbp_spell_kayn)))))
        (:`CastFailed`
          (bind _asbp_spell_kayn_spirit (cast `/Game/Winged/Blueprints/Effects/BP_Spell_KaynSpirit` OtherActor))
          (`self.K2_DestroyActor` _asbp_spell_kayn_spirit)
          (`KismetArrayLibrary.Array_Add` (`/Game/Winged/Blueprints/WingedSaveGame.Events_MultiplayerInteraction` (`/Game/Winged/Blueprints/WingedGameInstance.SaveGame` (cast `/Game/Winged/Blueprints/WingedGameInstance` (`GameplayStatics.GetGameInstance`) :!pure true))) (make `/Game/Winged/Blueprints/Structure_Event` (`KismetSystemLibrary.GetGameTimeInSeconds`) (`self.K2_GetActorLocation`) (`/Game/Winged/Blueprints/Kora.CurrentRespawnLocation` (cast `/Game/Winged/Blueprints/Kora` (`self.GetOwner`) :!pure true)) (`KismetStringLibrary.Concat_StrStr` (`KismetSystemLibrary.GetDisplayName` self) (`KismetSystemLibrary.GetDisplayName` _asbp_spell_kayn_spirit)))))))))

(fn `UserConstructionScript`)