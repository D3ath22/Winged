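; Kayn's spell effect, a short-lived aura actor that counters Kora and her spells before destroying itself after a fixed delay.
; On overlap, the Aura component stuns Kora or destroys her Spell and SpiritSpell actors.
; Each such hit is appended to the save game's multiplayer interaction events with game time, location, the owning Kayn's respawn location and both actors' names.
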(event `self.ReceiveBeginPlay`
  (`KismetSystemLibrary.Delay` 3.0)
  (`self.K2_DestroyActor`))

(event `self.Aura.OnComponentBeginOverlap`
  (params (OverlappedComponent :type "PrimitiveComponent Object Reference") (OtherActor :type "Actor Object Reference") (OtherComp :type "PrimitiveComponent Object Reference") (OtherBodyIndex :type Integer) (bFromSweep :type Boolean) (SweepResult :type "HitResult Structure (by ref)"))
  (bind _askora (cast `/Game/Winged/Blueprints/Kora` OtherActor)
    (:`then`
      (`/Game/Winged/Blueprints/Kora.Stun` _askora)
      (`KismetArrayLibrary.Array_Add` (`/Game/Winged/Blueprints/WingedSaveGame.Events_MultiplayerInteraction` (`/Game/Winged/Blueprints/WingedGameInstance.SaveGame` (cast `/Game/Winged/Blueprints/WingedGameInstance` (`GameplayStatics.GetGameInstance`) :!pure true))) (make `/Game/Winged/Blueprints/Structure_Event` (`KismetSystemLibrary.GetGameTimeInSeconds`) (`self.K2_GetActorLocation`) (`/Game/Winged/Blueprints/Kayn.CurrentRespawnLocation` (cast `/Game/Winged/Blueprints/Kayn` (`self.GetOwner`) :!pure true)) (`KismetStringLibrary.Concat_StrStr` (`KismetSystemLibrary.GetDisplayName` self) (`KismetSystemLibrary.GetDisplayName` _askora)))))
    (:`CastFailed`
      (bind _asbp_spell_kora (cast `/Game/Winged/Blueprints/Effects/BP_Spell_Kora` OtherActor)
        (:`then`
          (`self.K2_DestroyActor` _asbp_spell_kora)
          (`KismetArrayLibrary.Array_Add` (`/Game/Winged/Blueprints/WingedSaveGame.Events_MultiplayerInteraction` (`/Game/Winged/Blueprints/WingedGameInstance.SaveGame` (cast `/Game/Winged/Blueprints/WingedGameInstance` (`GameplayStatics.GetGameInstance`) :!pure true))) (make `/Game/Winged/Blueprints/Structure_Event` (`KismetSystemLibrary.GetGameTimeInSeconds`) (`self.K2_GetActorLocation`) (`/Game/Winged/Blueprints/Kayn.CurrentRespawnLocation` (cast `/Game/Winged/Blueprints/Kayn` (`self.GetOwner`) :!pure true)) (`KismetStringLibrary.Concat_StrStr` (`KismetSystemLibrary.GetDisplayName` self) (`KismetSystemLibrary.GetDisplayName` _asbp_spell_kora)))))
        (:`CastFailed`
          (bind _asbp_spell_kora_spirit (cast `/Game/Winged/Blueprints/Effects/BP_Spell_KoraSpirit` OtherActor))
          (`self.K2_DestroyActor` _asbp_spell_kora_spirit)
          (`KismetArrayLibrary.Array_Add` (`/Game/Winged/Blueprints/WingedSaveGame.Events_MultiplayerInteraction` (`/Game/Winged/Blueprints/WingedGameInstance.SaveGame` (cast `/Game/Winged/Blueprints/WingedGameInstance` (`GameplayStatics.GetGameInstance`) :!pure true))) (make `/Game/Winged/Blueprints/Structure_Event` (`KismetSystemLibrary.GetGameTimeInSeconds`) (`self.K2_GetActorLocation`) (`/Game/Winged/Blueprints/Kayn.CurrentRespawnLocation` (cast `/Game/Winged/Blueprints/Kayn` (`self.GetOwner`) :!pure true)) (`KismetStringLibrary.Concat_StrStr` (`KismetSystemLibrary.GetDisplayName` self) (`KismetSystemLibrary.GetDisplayName` _asbp_spell_kora_spirit)))))))))

(fn `UserConstructionScript`)