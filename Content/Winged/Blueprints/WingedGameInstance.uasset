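; Game instance for Winged that owns save data: a shared CommonSaveGame slot and numbered per-test saves.
; Init creates or loads the common save, whose counter names each new test slot; PrintTests dumps logged interaction and action events from those slots on screen.
; Save records Kora or Kayn scores per level in the test slot, while leaderboard entries go to the common save.
; OrderLeaderboard selection-sorts both levels by ascending time without writing to disk.
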(event `self.ReceiveInit`
  (bind _returnvalue (`GameplayStatics.DoesSaveGameExist` "CommonSaveGame"))
  (if (not _returnvalue)
    (bind _returnvalue_2 (`GameplayStatics.CreateSaveGameObject` "/Game/Winged/Blueprints/WingedSaveGame.WingedSaveGame_C"))
    (`GameplayStatics.SaveGameToSlot` _returnvalue_2 "CommonSaveGame"))
  (bind _returnvalue_3 (`GameplayStatics.LoadGameFromSlot` "CommonSaveGame"))
  (bind _aswinged_save_game (cast `/Game/Winged/Blueprints/WingedSaveGame` _returnvalue_3))
  (set `self.CommonSaveGame` _aswinged_save_game))

(event `NewTest`
  (bind _commonsavegame (`self.CommonSaveGame`))
  (bind _testnumber (`/Game/Winged/Blueprints/WingedSaveGame.TestNumber` _commonsavegame))
  ;[1 1 1] New Test
  (bind _returnvalue (`GameplayStatics.CreateSaveGameObject` "/Game/Winged/Blueprints/WingedSaveGame.WingedSaveGame_C"))
  (bind _output_get (set `self.SaveGame` _returnvalue))
  (bind _output_get_2 (set `/Game/Winged/Blueprints/WingedSaveGame.TestNumber` _testnumber _output_get))
  (bind _output_get_3 (set `self.SaveGameName` (`KismetStringLibrary.Concat_StrStr` (`self.SaveGameNameBase`) (`KismetStringLibrary.Conv_IntToString` _output_get_2))))
  (`GameplayStatics.SaveGameToSlot` _output_get _output_get_3)
  (set `/Game/Winged/Blueprints/WingedSaveGame.TestNumber` (+ _testnumber 1) _commonsavegame)
  (`GameplayStatics.SaveGameToSlot` _commonsavegame "CommonSaveGame"))

(event `PrintTests`
  ;[1 1 1] Print Tests
  (for _index (range 1001)
    (bind _returnvalue (`KismetStringLibrary.Concat_StrStr` (`self.SaveGameNameBase`) (`KismetStringLibrary.Conv_IntToString` _index)))
    (bind _returnvalue_2 (`GameplayStatics.DoesSaveGameExist` _returnvalue))
    (if _returnvalue_2
      (bind _returnvalue_3 (`GameplayStatics.LoadGameFromSlot` _returnvalue))
      (bind _aswinged_save_game (cast `/Game/Winged/Blueprints/WingedSaveGame` _returnvalue_3))
      (`KismetSystemLibrary.PrintString` (`KismetStringLibrary.Conv_IntToString` (`/Game/Winged/Blueprints/WingedSaveGame.TestNumber` _aswinged_save_game)) true true (struct :`G` 0.66 :`B` 1.0 :`A` 1.0) 10.0)
      (for _array_element (`/Game/Winged/Blueprints/WingedSaveGame.Events_SingleplayerInteraction` _aswinged_save_game)
        (`KismetSystemLibrary.PrintString` (`KismetStringLibrary.Conv_DoubleToString` (break `/Game/Winged/Blueprints/Structure_Event` _array_element)) true true (struct :`G` 0.66 :`B` 1.0 :`A` 1.0) 10.0)
        (`KismetSystemLibrary.PrintString` (`KismetStringLibrary.Conv_VectorToString` (`.Location_5_575EC5414F03535DA93F66843D3921ED` (break `/Game/Winged/Blueprints/Structure_Event` _array_element))) true true (struct :`G` 0.66 :`B` 1.0 :`A` 1.0) 10.0)
        (`KismetSystemLibrary.PrintString` (`KismetStringLibrary.Conv_IntToString` (`.Section_8_04FAE2F84C4E9F666DF5A8863EB6B0B4` (break `/Game/Winged/Blueprints/Structure_Event` _array_element))) true true (struct :`G` 0.66 :`B` 1.0 :`A` 1.0) 10.0)
        (`KismetSystemLibrary.PrintString` (`.Object_12_5A977868468C88043FDC03A174D58CCB` (break `/Game/Winged/Blueprints/Structure_Event` _array_element)) true true (struct :`G` 0.66 :`B` 1.0 :`A` 1.0) 10.0))
      (for _array_element_2 (`/Game/Winged/Blueprints/WingedSaveGame.Events_MultiplayerInteraction` _aswinged_save_game)
        (`KismetSystemLibrary.PrintString` (`KismetStringLibrary.Conv_DoubleToString` (break `/Game/Winged/Blueprints/Structure_Event` _array_element_2)) true true (struct :`G` 0.66 :`B` 1.0 :`A` 1.0) 10.0)
        (`KismetSystemLibrary.PrintString` (`KismetStringLibrary.Conv_VectorToString` (`.Location_5_575EC5414F03535DA93F66843D3921ED` (break `/Game/Winged/Blueprints/Structure_Event` _array_element_2))) true true (struct :`G` 0.66 :`B` 1.0 :`A` 1.0) 10.0)
        (`KismetSystemLibrary.PrintString` (`KismetStringLibrary.Conv_IntToString` (`.Section_8_04FAE2F84C4E9F666DF5A8863EB6B0B4` (break `/Game/Winged/Blueprints/Structure_Event` _array_element_2))) true true (struct :`G` 0.66 :`B` 1.0 :`A` 1.0) 10.0)
        (`KismetSystemLibrary.PrintString` (`.Object_12_5A977868468C88043FDC03A174D58CCB` (break `/Game/Winged/Blueprints/Structure_Event` _array_element_2)) true true (struct :`G` 0.66 :`B` 1.0 :`A` 1.0) 10.0))
      (for _array_element_3 (`/Game/Winged/Blueprints/WingedSaveGame.Events_Actions` _aswinged_save_game)
        (`KismetSystemLibrary.PrintString` (`KismetStringLibrary.Conv_DoubleToString` (break `/Game/Winged/Blueprints/Structure_Event` _array_element_3)) true true (struct :`G` 0.66 :`B` 1.0 :`A` 1.0) 10.0)
        (`KismetSystemLibrary.PrintString` (`KismetStringLibrary.Conv_VectorToString` (`.Location_5_575EC5414F03535DA93F66843D3921ED` (break `/Game/Winged/Blueprints/Structure_Event` _array_element_3))) true true (struct :`G` 0.66 :`B` 1.0 :`A` 1.0) 10.0)
        (`KismetSystemLibrary.PrintString` (`KismetStringLibrary.Conv_IntToString` (`.Section_8_04FAE2F84C4E9F666DF5A8863EB6B0B4` (break `/Game/Winged/Blueprints/Structure_Event` _array_element_3))) true true (struct :`G` 0.66 :`B` 1.0 :`A` 1.0) 10.0)
        (`KismetSystemLibrary.PrintString` (`.Object_12_5A977868468C88043FDC03A174D58CCB` (break `/Game/Winged/Blueprints/Structure_Event` _array_element_3)) true true (struct :`G` 0.66 :`B` 1.0 :`A` 1.0) 10.0))
      (else
        (break)))))

(fn `AddToLeaderboard`
  (params (Name :type String) (Time :type "Float (double-precision)"))
  (bind _commonsavegame (`self.CommonSaveGame`))
  (if (`KismetStringLibrary.EqualEqual_StrStr` (`self.Level`) "LevelOne")
    (`KismetArrayLibrary.Array_Add` (`/Game/Winged/Blueprints/WingedSaveGame.LevelOneLeaderboard_Names` _commonsavegame) Name)
    (`KismetArrayLibrary.Array_Add` (`/Game/Winged/Blueprints/WingedSaveGame.LevelOneLeaderboard_Times` _commonsavegame) Time)
    (else
      (`KismetArrayLibrary.Array_Add` (`/Game/Winged/Blueprints/WingedSaveGame.LevelTwoLeaderboard_Names` _commonsavegame) Name)
      (`KismetArrayLibrary.Array_Add` (`/Game/Winged/Blueprints/WingedSaveGame.LevelTwoLeaderboard_Times` _commonsavegame) Time)))
  (`GameplayStatics.SaveGameToSlot` _commonsavegame "CommonSaveGame"))

(fn `OrderLeaderboard`
  (locals (TimesTemp :type "Array of Float (double-precision)") (NamesTemp :type "Array of String"))
  (bind _commonsavegame (`self.CommonSaveGame`))
  (bind _timestemp (`local.TimesTemp`))
  (bind _namestemp (`local.NamesTemp`))
  (bind _timestemp_2 (`local.TimesTemp`))
  (bind _namestemp_2 (`local.NamesTemp`))
  (bind _commonsavegame_2 (`self.CommonSaveGame`))
  (bind _leveloneleaderboard_times (`/Game/Winged/Blueprints/WingedSaveGame.LevelOneLeaderboard_Times` _commonsavegame_2))
  (bind _leveloneleaderboard_names (`/Game/Winged/Blueprints/WingedSaveGame.LevelOneLeaderboard_Names` _commonsavegame_2))
  (bind _leveltwoleaderboard_times (`/Game/Winged/Blueprints/WingedSaveGame.LevelTwoLeaderboard_Times` _commonsavegame))
  (bind _leveltwoleaderboard_names (`/Game/Winged/Blueprints/WingedSaveGame.LevelTwoLeaderboard_Names` _commonsavegame))
  (bind (_indexofminvalue _minvalue) (`KismetMathLibrary.MinOfFloatArray` _leveloneleaderboard_times))
  (bind (_indexofminvalue_2 _minvalue_2) (`KismetMathLibrary.MinOfFloatArray` _leveltwoleaderboard_times))
  (while (> (`KismetArrayLibrary.Array_Length` _leveloneleaderboard_times) 0)
    (`KismetArrayLibrary.Array_Add` _timestemp_2 _minvalue)
    (`KismetArrayLibrary.Array_Add` _namestemp_2 (`|GetArrayItem` _leveloneleaderboard_names _indexofminvalue))
    (`KismetArrayLibrary.Array_Remove` _leveloneleaderboard_names _indexofminvalue)
    (`KismetArrayLibrary.Array_Remove` _leveloneleaderboard_times _indexofminvalue))
  (set `/Game/Winged/Blueprints/WingedSaveGame.LevelOneLeaderboard_Times` _timestemp_2 _commonsavegame_2)
  (set `/Game/Winged/Blueprints/WingedSaveGame.LevelOneLeaderboard_Names` _namestemp_2 _commonsavegame_2)
  (`KismetArrayLibrary.Array_Clear` (`local.TimesTemp`))
  (`KismetArrayLibrary.Array_Clear` (`local.NamesTemp`))
  (while (> (`KismetArrayLibrary.Array_Length` _leveltwoleaderboard_times) 0)
    (`KismetArrayLibrary.Array_Add` _timestemp _minvalue_2)
    (`KismetArrayLibrary.Array_Add` _namestemp (`|GetArrayItem` _leveltwoleaderboard_names _indexofminvalue_2))
    (`KismetArrayLibrary.Array_Remove` _leveltwoleaderboard_names _indexofminvalue_2)
    (`KismetArrayLibrary.Array_Remove` _leveltwoleaderboard_times _indexofminvalue_2))
  (set `/Game/Winged/Blueprints/WingedSaveGame.LevelTwoLeaderboard_Times` _timestemp _commonsavegame)
  (set `/Game/Winged/Blueprints/WingedSaveGame.LevelTwoLeaderboard_Names` _namestemp _commonsavegame))

(fn `Save`
  (params (Score :type String) (Kora :type Boolean))
  (bind _savegame (`self.SaveGame`))
  (if (`KismetStringLibrary.EqualEqual_StrStr` (`self.Level`) "LevelOne")
    (if Kora
      (set `/Game/Winged/Blueprints/WingedSaveGame.LevelOneKoraScore` Score _savegame)
      (else
        (set `/Game/Winged/Blueprints/WingedSaveGame.LevelOneKaynScore` Score _savegame)))
    (elif Kora
      (set `/Game/Winged/Blueprints/WingedSaveGame.LevelTwoKoraScore` Score _savegame)
      (else
        (set `/Game/Winged/Blueprints/WingedSaveGame.LevelTwoKaynScore` Score _savegame))))
  (`GameplayStatics.SaveGameToSlot` _savegame (`self.SaveGameName`)))