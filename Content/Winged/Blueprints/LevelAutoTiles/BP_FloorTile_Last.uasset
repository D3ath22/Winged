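; Final auto-tile floor piece that ends a Winged run when Kora or Kayn overlaps its Portal_Fragment.
; The portal stamps that character's finish time, records the first finisher as winner in WingedGameInstance, and shows KoraTransitionMenuWidget.
; Either wall kills Kora when the hit normal nearly matches Kora's forward vector.
; Helper functions expose the attach transform and randomly place blockers, tea leaves and neon, though nothing here calls them.
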(event `self.ReceiveTick`
  (params (DeltaSeconds :type "Float (single-precision)")))

(event `self.Portal_Fragment.OnComponentBeginOverlap`
  (params (OverlappedComponent :type "PrimitiveComponent Object Reference") (OtherActor :type "Actor Object Reference") (OtherComp :type "PrimitiveComponent Object Reference") (OtherBodyIndex :type Integer) (bFromSweep :type Boolean) (SweepResult :type "HitResult Structure (by ref)"))
  (bind _returnvalue (`KismetSystemLibrary.GetGameTimeInSeconds`))
  (bind _askora (cast `/Game/Winged/Blueprints/Kora` OtherActor)
    (:`then`
      (set `/Game/Winged/Blueprints/Kora.FinishTIme` _returnvalue _askora)
      (bind _aswinged_game_instance (cast `/Game/Winged/Blueprints/WingedGameInstance` (`GameplayStatics.GetGameInstance`)))
      (if (not (`/Game/Winged/Blueprints/WingedGameInstance.EndReached` _aswinged_game_instance))
        (set `/Game/Winged/Blueprints/WingedGameInstance.KoraWin` true _aswinged_game_instance)
        (set `/Game/Winged/Blueprints/WingedGameInstance.EndReached` true _aswinged_game_instance)))
    (:`CastFailed`
      (bind _askayn (cast `/Game/Winged/Blueprints/Kayn` OtherActor))
      (set `/Game/Winged/Blueprints/Kayn.FinishTime` _returnvalue _askayn)
      (bind _aswinged_game_instance_2 (cast `/Game/Winged/Blueprints/WingedGameInstance` (`GameplayStatics.GetGameInstance`)))
      (if (not (`/Game/Winged/Blueprints/WingedGameInstance.EndReached` _aswinged_game_instance_2))
        (set `/Game/Winged/Blueprints/WingedGameInstance.KoraWin` false _aswinged_game_instance_2)
        (set `/Game/Winged/Blueprints/WingedGameInstance.EndReached` true _aswinged_game_instance_2))))
  (bind _returnvalue_2 (`|CreateWidget` "/Game/Winged/Blueprints/TransitionMenu/KoraTransitionMenuWidget.KoraTransitionMenuWidget_C"))
  (`UserWidget.AddToViewport` _returnvalue_2 1))

(event `self.Wall.OnComponentHit`
  (params (HitComponent :type "PrimitiveComponent Object Reference") (OtherActor :type "Actor Object Reference") (OtherComp :type "PrimitiveComponent Object Reference") (NormalImpulse :type "Vector Structure") (Hit :type "HitResult Structure (by ref)"))
  ;[1 1 1] Hit Wall Straight On
  (bind _askora (cast `/Game/Winged/Blueprints/Kora` OtherActor))
  (if (`KismetMathLibrary.NearlyEqual_FloatFloat` (`KismetMathLibrary.Dot_VectorVector` Hit_Normal (`self.GetActorForwardVector` _askora)) 1.0 0.01)
    (`/Game/Winged/Blueprints/Kora.Death` _askora)))

(event `self.Wall2.OnComponentHit`
  (params (HitComponent :type "PrimitiveComponent Object Reference") (OtherActor :type "Actor Object Reference") (OtherComp :type "PrimitiveComponent Object Reference") (NormalImpulse :type "Vector Structure") (Hit :type "HitResult Structure (by ref)"))
  ;[1 1 1] Hit Wall Straight On
  (bind _askora (cast `/Game/Winged/Blueprints/Kora` OtherActor))
  (if (`KismetMathLibrary.NearlyEqual_FloatFloat` (`KismetMathLibrary.Dot_VectorVector` Hit_Normal (`self.GetActorForwardVector` _askora)) 1.0 0.01)
    (`/Game/Winged/Blueprints/Kora.Death` _askora)))

(fn `GetAttachTransform`
  (returns (AttachTransform :type "Transform Structure"))
  (return (`SceneComponent.K2_GetComponentToWorld` (`self.AttachPoint`))))

(fn `SetSpawnPoints`
  (set `self.SpawnPoints` (`|MakeArray` (`SceneComponent.GetRelativeTransform` (`self.SpawnPointTopLeft`)) (`SceneComponent.GetRelativeTransform` (`self.SpawnPointTopCenter`)) (`SceneComponent.GetRelativeTransform` (`self.SpawnPointTopRight`)) (`SceneComponent.GetRelativeTransform` (`self.SpawnPointBottomLeft`)) (`SceneComponent.GetRelativeTransform` (`self.SpawnPointBottomCenter`)) (`SceneComponent.GetRelativeTransform` (`self.SpawnPointBottomRIght`)))))

(fn `SpawnBlocker`
  (bind _spawnpoints (`self.SpawnPoints`))
  (bind _blockertypes (`self.BlockerTypes`))
  (bind _returnvalue (`AddComponent|NODE_AddChildActorComponent-0` :`RelativeTransform` (`|GetArrayItem` _spawnpoints (`KismetMathLibrary.RandomIntegerInRange` 0 (`KismetArrayLibrary.Array_LastIndex` _spawnpoints)))))
  (`ChildActorComponent.SetChildActorClass` _returnvalue (`|GetArrayItem` _blockertypes (`KismetMathLibrary.RandomIntegerInRange` 0 (`KismetArrayLibrary.Array_LastIndex` _blockertypes)))))

(fn `SpawnNeon`
  (bind _neonarearight (`self.NeonAreaRight`))
  (bind _neonarealeft (`self.NeonAreaLeft`))
  (if (`KismetMathLibrary.RandomBool`)
    (for _ (range (+ (`KismetMathLibrary.RandomIntegerInRange` 1 1) 1))
      (`AddComponent|NODE_AddChildActorComponent-7` :`RelativeTransform` (`KismetMathLibrary.Conv_VectorToTransform` (`KismetMathLibrary.RandomPointInBoundingBox` (`SceneComponent.RelativeLocation` _neonarearight) (`BoxComponent.BoxExtent` _neonarearight)))))
    (else
      (for _ (range (+ (`KismetMathLibrary.RandomIntegerInRange` 1 1) 1))
        (`AddComponent|NODE_AddChildActorComponent-8` :`RelativeTransform` (`KismetMathLibrary.Conv_VectorToTransform` (`KismetMathLibrary.RandomPointInBoundingBox` (`SceneComponent.RelativeLocation` _neonarealeft) (`BoxComponent.BoxExtent` _neonarealeft))))))))

(fn `SpawnTeaLeaves`
  (bind _tealeavesarealeft (`self.TeaLeavesAreaLeft`))
  (bind _tealeavesarearight (`self.TeaLeavesAreaRight`))
  (if (`KismetMathLibrary.RandomBool`)
    (for _ (range (+ (`KismetMathLibrary.RandomIntegerInRange` 1 3) 1))
      (`AddComponent|NODE_AddChildActorComponent-2` :`RelativeTransform` (`KismetMathLibrary.Conv_VectorToTransform` (`KismetMathLibrary.RandomPointInBoundingBox` (`SceneComponent.RelativeLocation` _tealeavesarearight) (`BoxComponent.BoxExtent` _tealeavesarearight)))))
    (else
      (for _ (range (+ (`KismetMathLibrary.RandomIntegerInRange` 1 3) 1))
        (`AddComponent|NODE_AddChildActorComponent-1` :`RelativeTransform` (`KismetMathLibrary.Conv_VectorToTransform` (`KismetMathLibrary.RandomPointInBoundingBox` (`SceneComponent.RelativeLocation` _tealeavesarealeft) (`BoxComponent.BoxExtent` _tealeavesarealeft))))))))

(fn `UserConstructionScript`)