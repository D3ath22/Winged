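; Floor tile for an endless-runner style level, exposing an attach transform and asking WingedGameMode to add another tile when Kora or Kayn overlaps its end trigger.
; The construction script randomly adds either a blocker at one of six spawn points, or tea leaves or neon inside left or right boxes.
; Wall hits stun the characters when the hit normal aligns with a forward vector.
; Jump and interact spawners exist but are unused.
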(event `self.ReceiveTick`
  (params (DeltaSeconds :type "Float (single-precision)")))

(event `self.EndTrigger.OnComponentBeginOverlap`
  (params (OverlappedComponent :type "PrimitiveComponent Object Reference") (OtherActor :type "Actor Object Reference") (OtherComp :type "PrimitiveComponent Object Reference") (OtherBodyIndex :type Integer) (bFromSweep :type Boolean) (SweepResult :type "HitResult Structure (by ref)"))
  (cast `/Game/Winged/Blueprints/Kora` OtherActor
    (:`then`
      _)
    (:`CastFailed`
      (cast `/Game/Winged/Blueprints/Kayn` OtherActor)))
  (bind _aswinged_game_mode (cast `/Game/Winged/Blueprints/WingedGameMode` (`GameplayStatics.GetGameMode`)))
  (`/Game/Winged/Blueprints/WingedGameMode.AddFloorTile` _aswinged_game_mode))

(event `self.Wall.OnComponentHit`
  (params (HitComponent :type "PrimitiveComponent Object Reference") (OtherActor :type "Actor Object Reference") (OtherComp :type "PrimitiveComponent Object Reference") (NormalImpulse :type "Vector Structure") (Hit :type "HitResult Structure (by ref)"))
  ;[1 1 1] Hit Wall Straight On
  (bind _askora (cast `/Game/Winged/Blueprints/Kora` OtherActor)
    (:`then`
      (if (`KismetMathLibrary.NearlyEqual_FloatFloat` (`KismetMathLibrary.Dot_VectorVector` Hit_Normal (`self.GetActorForwardVector` _askora)) 1.0 0.01)
        (`/Game/Winged/Blueprints/Kora.Stun` _askora)))
    (:`CastFailed`
      (bind _askayn (cast `/Game/Winged/Blueprints/Kayn` OtherActor))
      (if (`KismetMathLibrary.NearlyEqual_FloatFloat` (`KismetMathLibrary.Dot_VectorVector` Hit_Normal (`self.GetActorForwardVector`)) 1.0 0.01)
        (`/Game/Winged/Blueprints/Kayn.Stun` _askayn)))))

(event `self.Wall2.OnComponentHit`
  (params (HitComponent :type "PrimitiveComponent Object Reference") (OtherActor :type "Actor Object Reference") (OtherComp :type "PrimitiveComponent Object Reference") (NormalImpulse :type "Vector Structure") (Hit :type "HitResult Structure (by ref)"))
  ;[1 1 1] Hit Wall Straight On
  (bind _askora (cast `/Game/Winged/Blueprints/Kora` OtherActor)
    (:`then`
      (if (`KismetMathLibrary.NearlyEqual_FloatFloat` (`KismetMathLibrary.Dot_VectorVector` Hit_Normal (`self.GetActorForwardVector` _askora)) 1.0 0.01)
        (`/Game/Winged/Blueprints/Kora.Stun` _askora)))
    (:`CastFailed`
      (bind _askayn (cast `/Game/Winged/Blueprints/Kayn` OtherActor))
      (if (`KismetMathLibrary.NearlyEqual_FloatFloat` (`KismetMathLibrary.Dot_VectorVector` Hit_Normal (`self.GetActorForwardVector` _askayn)) 1.0 0.01)
        (`/Game/Winged/Blueprints/Kayn.Stun` _askayn)))))

(fn `GetAttachTransform`
  (returns (AttachTransform :type "Transform Structure"))
  (return (`SceneComponent.K2_GetComponentToWorld` (`self.AttachPoint`))))

(fn `SetSpawnPoints`
  (set `self.SpawnPoints` (`|MakeArray` (`SceneComponent.GetRelativeTransform` (`self.SpawnPointTopLeft`)) (`SceneComponent.GetRelativeTransform` (`self.SpawnPointTopCenter`)) (`SceneComponent.GetRelativeTransform` (`self.SpawnPointTopRight`)) (`SceneComponent.GetRelativeTransform` (`self.SpawnPointBottomLeft`)) (`SceneComponent.GetRelativeTransform` (`self.SpawnPointBottomCenter`)) (`SceneComponent.GetRelativeTransform` (`self.SpawnPointBottomRIght`)))))

(fn `SpawnBlocker`
  (bind _spawnpoints (`self.SpawnPoints`))
  (bind _blockertypes (`self.BlockerTypes`))
  (bind _returnvalue (`AddComponent|NODE_AddChildActorComponent-0` :`RelativeTransform` (`|GetArrayItem` _spawnpoints (`KismetMathLibrary.RandomIntegerInRange` 0 (`KismetArrayLibrary.Array_LastIndex` _spawnpoints)))))
  (`ChildActorComponent.SetChildActorClass` _returnvalue (`|GetArrayItem` _blockertypes (`KismetMathLibrary.RandomIntegerInRange` 0 (`KismetArrayLibrary.Array_LastIndex` _blockertypes)))))

(fn `SpawnInteract`
  (bind _returnvalue (`SceneComponent.GetRelativeTransform` (`self.SpawnPointMiddleHigh`)))
  (switch `int` (`KismetMathLibrary.RandomIntegerInRange` 0 2)
    (:`0`
      (`AddComponent|NODE_AddChildActorComponent-12` :`RelativeTransform` _returnvalue))
    (:`1`
      (`AddComponent|NODE_AddChildActorComponent-14` :`RelativeTransform` _returnvalue))
    (:`2`
      (`AddComponent|NODE_AddChildActorComponent-15` :`RelativeTransform` _returnvalue)
      (`AddComponent|NODE_AddChildActorComponent-16` :`RelativeTransform` _returnvalue))))

(fn `SpawnJumps`
  (if (`KismetMathLibrary.RandomBool`)
    (`AddComponent|NODE_AddChildActorComponent-10` :`RelativeTransform` (`SceneComponent.GetRelativeTransform` (`self.SpawnPointMiddle`)))
    (else
      (`AddComponent|NODE_AddChildActorComponent-13` :`RelativeTransform` (`SceneComponent.GetRelativeTransform` (`self.SpawnPointMiddle`))))))

(fn `SpawnNeon`
  (bind _neonarearight (`self.NeonAreaRight`))
  (bind _neonarealeft (`self.NeonAreaLeft`))
  (if (`KismetMathLibrary.RandomBool`)
    (for _ (range (+ (`KismetMathLibrary.RandomIntegerInRange` 1 1) 1))
      (`AddComponent|NODE_AddChildActorComponent-7` :`RelativeTransform` (`KismetMathLibrary.Conv_VectorToTransform` (`KismetMathLibrary.RandomPointInBoundingBox` (`SceneComponent.RelativeLocation` _neonarearight) (`BoxComponent.BoxExtent` _neonarearight)))))
    (else
      (for _ (range (+ (`KismetMathLibrary.RandomIntegerInRange` 1 1) 1))
        (`AddComponent|NODE_AddChildActorComponent-8` :`RelativeTransform` (`KismetMathLibrary.Conv_VectorToTransform` (`KismetMathLibrary.RandomPointInBoundingBox` (`SceneComponent.RelativeLocation` _neonarealeft) (`BoxComponent.BoxExtent` _neonarealeft))))))))

(fn `SpawnTeaLeaves`
  (bind _tealeavesarealeft (`self.TeaLeavesAreaLeft`))
  (bind _tealeavesarearight (`self.TeaLeavesAreaRight`))
  (if (`KismetMathLibrary.RandomBool`)
    (for _ (range (+ (`KismetMathLibrary.RandomIntegerInRange` 1 3) 1))
      (`AddComponent|NODE_AddChildActorComponent-2` :`RelativeTransform` (`KismetMathLibrary.Conv_VectorToTransform` (`KismetMathLibrary.RandomPointInBoundingBox` (`SceneComponent.RelativeLocation` _tealeavesarearight) (`BoxComponent.BoxExtent` _tealeavesarearight)))))
    (else
      (for _ (range (+ (`KismetMathLibrary.RandomIntegerInRange` 1 3) 1))
        (`AddComponent|NODE_AddChildActorComponent-1` :`RelativeTransform` (`KismetMathLibrary.Conv_VectorToTransform` (`KismetMathLibrary.RandomPointInBoundingBox` (`SceneComponent.RelativeLocation` _tealeavesarealeft) (`BoxComponent.BoxExtent` _tealeavesarealeft))))))))

(fn `UserConstructionScript`
  (`self.SetSpawnPoints`)
  (switch `int` (`KismetMathLibrary.RandomIntegerInRange` 0 1)
    (:`Default`
      (`self.SpawnBlocker` :!label _label))
    (:`0`
      (goto _label))
    (:`1`
      (if (`KismetMathLibrary.RandomBool`)
        (`self.SpawnTeaLeaves`)
        (else
          (`self.SpawnNeon`))))))