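; Game mode for Winged that sets up one or two players as Kora or Kayn and builds the procedural track in LevelAuto.
; The game instance's settings pick each controller's pawn and HUD, creating a second local player outside single-player.
; On LevelAuto, BeginPlay seeds floor tiles by chaining attach transforms: random straights, curves after randomized runs, and special first and last pieces.
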(event `self.ReceiveBeginPlay`
  (bind _returnvalue (`GameplayStatics.GetPlayerController` 0))
  ;[1 1 1] Create player 2, ignore up, right for auto level
  (bind _aswinged_game_instance (cast `/Game/Winged/Blueprints/WingedGameInstance` (`GameplayStatics.GetGameInstance`)))
  (if (`/Game/Winged/Blueprints/WingedGameInstance.SinglePlayer` _aswinged_game_instance)
    (if (`/Game/Winged/Blueprints/WingedGameInstance.Kora` _aswinged_game_instance)
      (bind _returnvalue_2 (`|CreateWidget` "/Game/Winged/Blueprints/KoraHUD.KoraHUD_C" _returnvalue))
      (`UserWidget.AddToViewport` _returnvalue_2 0)
      (else
        (bind _returnvalue_3 (`|CreateWidget` "/Game/Winged/Blueprints/KaynHUD.KaynHUD_C" _returnvalue))
        (`UserWidget.AddToViewport` _returnvalue_3 0)))
    (bind _returnvalue_4 (`GameplayStatics.GetCurrentLevelName` true))
    (if (`KismetStringLibrary.EqualEqual_StrStr` _returnvalue_4 "LevelAuto")
      (for _ (range 10)
        (`self.AddFloorTile`)
        (bind _returnvalue_5 (`GameplayStatics.GetCurrentLevelName` true :!label _label))
        (if (`KismetStringLibrary.EqualEqual_StrStr` _returnvalue_5 "LevelAuto")
          (for _ (range 10)
            (`self.AddFloorTile`)))))
    (else
      (`GameplayStatics.CreatePlayer` 1)
      (bind _returnvalue_6 (`|CreateWidget` "/Game/Winged/Blueprints/KaynHUD.KaynHUD_C" (`GameplayStatics.GetPlayerController` 1)))
      (`UserWidget.AddToPlayerScreen` _returnvalue_6 0)
      (bind _returnvalue_7 (`|CreateWidget` "/Game/Winged/Blueprints/KoraHUD.KoraHUD_C" (`GameplayStatics.GetPlayerController` 0)))
      (`UserWidget.AddToPlayerScreen` _returnvalue_7 0)
      (bind _returnvalue_8 (`GameplayStatics.GetCurrentLevelName` true))
      (if (`KismetStringLibrary.EqualEqual_StrStr` _returnvalue_8 "LevelAuto")
        (for _ (range 10)
          (`self.AddFloorTile`)
          (goto _label))))))

(fn `AddFirstFloorTile`
  (bind _returnvalue (`|SpawnActorFromClass` "/Game/Winged/Blueprints/LevelAutoTiles/BP_FloorTile_First.BP_FloorTile_First_C" (`self.NextSpawnPoint`) "Undefined" "OverrideRootScale" null null))
  (bind _attachtransform (`/Game/Winged/Blueprints/LevelAutoTiles/BP_FloorTile.GetAttachTransform` _returnvalue))
  (set `self.NextSpawnPoint` _attachtransform)
  (set `self.CurrentStraights` (+ (`self.CurrentStraights`) 1))
  (set `self.FloorTilesCount` (+ (`self.FloorTilesCount`) 1)))

(fn `AddFloorCurve`
  (bind _floorcurves (`self.FloorCurves`))
  (bind _returnvalue (`|SpawnActorFromClass` (`|GetArrayItem` _floorcurves (`KismetMathLibrary.RandomIntegerInRange` 0 (`KismetArrayLibrary.Array_LastIndex` _floorcurves))) (`self.NextSpawnPoint`) "Undefined" "OverrideRootScale" null null))
  (bind _asbp_floor_tile (cast `/Game/Winged/Blueprints/LevelAutoTiles/BP_FloorTile` _returnvalue))
  (bind _attachtransform (`/Game/Winged/Blueprints/LevelAutoTiles/BP_FloorTile.GetAttachTransform` _asbp_floor_tile))
  (set `self.NextSpawnPoint` _attachtransform)
  (set `self.CurrentStraights` 0)
  (set `self.FloorTilesCount` (+ (`self.FloorTilesCount`) 1)))

(fn `AddFloorTile`
  (bind _floortiles (`self.FloorTiles`))
  (if (== (`self.FloorTilesCount`) 0)
    (`self.AddFirstFloorTile`)
    (elif (== (`self.FloorTilesCount`) 100)
      (`self.AddLastFloorTile`)
      (elif (> (`self.CurrentStraights`) (`KismetMathLibrary.RandomIntegerInRange` 9 19))
        (`self.AddFloorCurve`)
        (else
          (bind _returnvalue (`|SpawnActorFromClass` (`|GetArrayItem` _floortiles (`KismetMathLibrary.RandomIntegerInRange` 0 (`KismetArrayLibrary.Array_LastIndex` _floortiles))) (`self.NextSpawnPoint`) "Undefined" "OverrideRootScale" null null))
          (bind _asbp_floor_tile (cast `/Game/Winged/Blueprints/LevelAutoTiles/BP_FloorTile` _returnvalue))
          (bind _attachtransform (`/Game/Winged/Blueprints/LevelAutoTiles/BP_FloorTile.GetAttachTransform` _asbp_floor_tile))
          (set `self.NextSpawnPoint` _attachtransform)
          (set `self.CurrentStraights` (+ (`self.CurrentStraights`) 1))
          (set `self.FloorTilesCount` (+ (`self.FloorTilesCount`) 1)))))))

(fn `AddLastFloorTile`
  (`|SpawnActorFromClass` "/Game/Winged/Blueprints/LevelAutoTiles/BP_FloorTile_Last.BP_FloorTile_Last_C" (`self.NextSpawnPoint`) "Undefined" "OverrideRootScale" null null))

(fn `GetDefaultPawnClassForController`
  (params (InController :type "Controller Object Reference"))
  (returns (ReturnValue :type "Object Class Reference"))
  (`parent.GetDefaultPawnClassForController` InController)
  (bind _aswinged_game_instance (cast `/Game/Winged/Blueprints/WingedGameInstance` (`GameplayStatics.GetGameInstance`)))
  (if (`/Game/Winged/Blueprints/WingedGameInstance.SinglePlayer` _aswinged_game_instance)
    (if (`/Game/Winged/Blueprints/WingedGameInstance.Kora` _aswinged_game_instance)
      (bind _output_get (set `self.DefaultPawnClass` "/Game/Winged/Blueprints/Kora.Kora_C"))
      (return _output_get)
      (else
        (bind _output_get_2 (set `self.DefaultPawnClass` "/Game/Winged/Blueprints/Kayn.Kayn_C"))
        (return _output_get_2)))
    (else
      (bind _asplayer_controller (cast `PlayerController` InController))
      (if (== (`GameplayStatics.GetPlayerControllerID` _asplayer_controller) 0)
        (bind _output_get_3 (set `self.DefaultPawnClass` "/Game/Winged/Blueprints/Kora.Kora_C"))
        (return _output_get_3)
        (else
          (bind _output_get_4 (set `self.DefaultPawnClass` "/Game/Winged/Blueprints/Kayn.Kayn_C"))
          (return _output_get_4))))))

(fn `UserConstructionScript`)